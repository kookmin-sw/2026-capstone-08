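; BP_Shopkeeper is a shopkeeper that stocks its shop with random weapons and runes on BeginPlay.
; The construction script collects two weapon and four rune points, where shop item actors are spawned.
; Each item gets data from the Mortis weapon or rune database subsystem, with the floor 1 argument hardcoded for weapons.
; Items are then tinted by grade color, given a generated price and linked back to the shopkeeper.
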(event EventBeginPlay
  (bind _returnvalue (Subsystems|GetMortisRuneDatabaseSubsystem))
  (Utilities|FlowControl|Sequence
    (:then_0
      (for _index (range 0 (- (Utilities|Array|Length (Variables|Default|GetWeaponPoints)) 1))
        (bind _returnvalue_2 (Game|SpawnActorfromClass "/Game/Items/ShopItem/BP_WeaponShopItem.BP_WeaponShopItem_C" (Transformation|GetWorldTransform (Utilities|Array|Get(acopy) (Variables|Default|GetWeaponPoints) _index)) "Undefined" "MultiplyWithRoot" 0 0))
        (Class|MortisWeaponPickup|SetWeaponData _returnvalue_2 (.OutWeaponRow (Class|MortisWeaponDatabaseSubsystem|GenerateRandomWeaponforFloor (Subsystems|GetMortisWeaponDatabaseSubsystem) 1)))
        (Rendering|Material|SetColorParameterValueonMaterials (Variables|/Script/EternalMortis.MortisInteractableActorBase|GetVisualMesh _returnvalue_2) "FresColor" (.GradeColor (Utilities|Struct|BreakMortisWeaponGradeStyleRow (.OutStyleRow (Class|MortisWeaponDatabaseSubsystem|GetWeaponGradeStylebyHandle (Subsystems|GetMortisWeaponDatabaseSubsystem) (.GradeStyleRow (Utilities|Struct|BreakMortisWeaponRow (Variables|/Script/EternalMortis.MortisWeaponPickup|GetWeaponData _returnvalue_2))))))))
        (Class|MortisShopkeeperCharacter|InitializeWeaponShopItemwithGeneratedPrice _returnvalue_2 (Variables|/Script/EternalMortis.MortisWeaponPickup|GetWeaponData _returnvalue_2))
        (Class|MortisWeaponShopItem|SetOwningShopkeeper _returnvalue_2 self)))
    (:then_1
      (for _index_2 (range 0 (- (Utilities|Array|Length (Variables|Default|GetRunePoints)) 1))
        (bind _returnvalue_3 (Game|SpawnActorfromClass "/Game/Items/ShopItem/BP_RuneShopItem.BP_RuneShopItem_C" (Transformation|GetWorldTransform (Utilities|Array|Get(acopy) (Variables|Default|GetRunePoints) _index_2)) "Undefined" "MultiplyWithRoot" 0 0))
        (Class|MortisRunePickup|SetRuneData _returnvalue_3 (Class|MortisRuneDatabaseSubsystem|GenerateRune _returnvalue 1))
        (Rendering|Material|SetColorParameterValueonMaterials (Variables|/Script/EternalMortis.MortisInteractableActorBase|GetVisualMesh _returnvalue_3) "FresColor" (.GradeColor (Utilities|Struct|BreakMortisRuneGradeStyleRow (.OutStyleRow (Class|MortisRuneDatabaseSubsystem|GetRuneGradeStylebyHandle _returnvalue (.GradeStyleRow (Utilities|Struct|BreakMortisRuneInstance (Variables|/Script/EternalMortis.MortisRunePickup|GetRuneData _returnvalue_3))))))))
        (Class|MortisShopkeeperCharacter|InitializeRuneShopItemwithGeneratedPrice _returnvalue_3 (Variables|/Script/EternalMortis.MortisRunePickup|GetRuneData _returnvalue_3))
        (Class|MortisRuneShopItem|SetOwningShopkeeper _returnvalue_3 self)))))

(event Collision|EventActorBeginOverlap
  (params (OtherActor :type Actor%20Object%20Reference)))

(event EventTick
  (params (DeltaSeconds :type Float%20%28single-precision%29)))

(fn ConstructionScript
  (bind _weaponpoints (Variables|Default|GetWeaponPoints))
  (Utilities|Array|Clear _weaponpoints)
  (Utilities|Array|Add _weaponpoints (Variables|Default|GetWeapon_01))
  (Utilities|Array|Add _weaponpoints (Variables|Default|GetWeapon_02))
  (Utilities|Array|Clear (Variables|Default|GetRunePoints))
  (Utilities|Array|Add (Variables|Default|GetRunePoints) (Variables|Default|GetRune_01))
  (Utilities|Array|Add (Variables|Default|GetRunePoints) (Variables|Default|GetRune_02))
  (Utilities|Array|Add (Variables|Default|GetRunePoints) (Variables|Default|GetRune_03))
  (Utilities|Array|Add (Variables|Default|GetRunePoints) (Variables|Default|GetRune_04)))