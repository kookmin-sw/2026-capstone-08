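; Secret helper actor that offers reward pickups at three spawn points when play begins.
; Spawns two rune pickups on the sides, plus a weapon pickup if the run state reports the true ending can be seen, otherwise an ending rune.
; Rune and weapon data are generated with a hardcoded floor-99 argument, and their grade color tints the pickup meshes.
; Each pickup is registered with the helper and linked back to it as owner.
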(event EventBeginPlay
  (bind _returnvalue (Subsystems|GetMortisRuneDatabaseSubsystem))
  (bind _returnvalue_2 (Subsystems|GetMortisRuneDatabaseSubsystem))
  (bind _returnvalue_3 (Subsystems|GetMortisWeaponDatabaseSubsystem))
  (bind _self self)
  (bind _self_2 self)
  (bind _pickupspawnpoint_0 (Variables|Default|GetPickupSpawnPoint_0))
  (bind _pickupspawnpoint_2 (Variables|Default|GetPickupSpawnPoint_2))
  (bind _pickupspawnpoint_1 (Variables|Default|GetPickupSpawnPoint_1))
  (bind _pickupspawnpoint_1_2 (Variables|Default|GetPickupSpawnPoint_1))
  (bind _returnvalue_4 (Transformation|GetWorldTransform _pickupspawnpoint_0))
  (bind _returnvalue_5 (Transformation|GetWorldTransform _pickupspawnpoint_1))
  (bind _returnvalue_6 (Transformation|GetWorldTransform _pickupspawnpoint_2))
  (bind _returnvalue_7 (Transformation|GetWorldTransform _pickupspawnpoint_1_2))
  (bind _returnvalue_8 (Game|SpawnActorfromClass "/Game/Items/PickUp/SecretHelper/BP_SecretHelperRunePickup.BP_SecretHelperRunePickup_C" (Math|Transform|MakeTransform (.location _returnvalue_4) (.rotation _returnvalue_4) "1.000000,1.000000,1.000000") "Undefined" "MultiplyWithRoot" 0 0))
  (Class|MortisRunePickup|SetRuneData _returnvalue_8 (Class|MortisRuneDatabaseSubsystem|GenerateRune _returnvalue_2 99))
  (Rendering|Material|SetColorParameterValueonMaterials (Variables|/Script/EternalMortis.MortisInteractableActorBase|GetVisualMesh _returnvalue_8) "FresColor" (.GradeColor (Utilities|Struct|BreakMortisRuneGradeStyleRow (.OutStyleRow (Class|MortisRuneDatabaseSubsystem|GetRuneGradeStylebyHandle _returnvalue_2 (.GradeStyleRow (Utilities|Struct|BreakMortisRuneInstance (Variables|/Script/EternalMortis.MortisRunePickup|GetRuneData _returnvalue_8))))))))
  (Class|MortisSecretHelper|RegisterOwnedPickup self _returnvalue_8)
  (Class|MortisSecretHelperRunePickup|SetOwningSecretHelper _returnvalue_8 self)
  (bind _returnvalue_9 (Game|SpawnActorfromClass "/Game/Items/PickUp/SecretHelper/BP_SecretHelperRunePickup.BP_SecretHelperRunePickup_C" (Math|Transform|MakeTransform (.location _returnvalue_6) (.rotation _returnvalue_6) "1.000000,1.000000,1.000000") "Undefined" "MultiplyWithRoot" 0 0))
  (Class|MortisRunePickup|SetRuneData _returnvalue_9 (Class|MortisRuneDatabaseSubsystem|GenerateRune _returnvalue 99))
  (Rendering|Material|SetColorParameterValueonMaterials (Variables|/Script/EternalMortis.MortisInteractableActorBase|GetVisualMesh _returnvalue_9) "FresColor" (.GradeColor (Utilities|Struct|BreakMortisRuneGradeStyleRow (.OutStyleRow (Class|MortisRuneDatabaseSubsystem|GetRuneGradeStylebyHandle _returnvalue (.GradeStyleRow (Utilities|Struct|BreakMortisRuneInstance (Variables|/Script/EternalMortis.MortisRunePickup|GetRuneData _returnvalue_9))))))))
  (Class|MortisSecretHelper|RegisterOwnedPickup self _returnvalue_9)
  (Class|MortisSecretHelperRunePickup|SetOwningSecretHelper _returnvalue_9 self)
  (if (Class|MortisRunStateSubsystem|CanSeeTrueEnding (Subsystems|GetMortisRunStateSubsystem))
    (bind _returnvalue_10 (Game|SpawnActorfromClass "/Game/Items/PickUp/SecretHelper/BP_SecretHelperWeaponPickup.BP_SecretHelperWeaponPickup_C" (Math|Transform|MakeTransform (.location _returnvalue_7) (.rotation _returnvalue_7) "1.000000,1.000000,1.000000") "Undefined" "MultiplyWithRoot" 0 0))
    (Class|MortisWeaponPickup|SetWeaponData _returnvalue_10 (.OutWeaponRow (Class|MortisWeaponDatabaseSubsystem|GenerateRandomWeaponforFloor _returnvalue_3 99)))
    (Rendering|Material|SetColorParameterValueonMaterials (Variables|/Script/EternalMortis.MortisInteractableActorBase|GetVisualMesh _returnvalue_10) "FresColor" (.GradeColor (Utilities|Struct|BreakMortisWeaponGradeStyleRow (.OutStyleRow (Class|MortisWeaponDatabaseSubsystem|GetWeaponGradeStylebyHandle _returnvalue_3 (.GradeStyleRow (Utilities|Struct|BreakMortisWeaponRow (Variables|/Script/EternalMortis.MortisWeaponPickup|GetWeaponData _returnvalue_10))))))))
    (Class|MortisSecretHelper|RegisterOwnedPickup _self _returnvalue_10)
    (Class|MortisSecretHelperWeaponPickup|SetOwningSecretHelper _returnvalue_10 _self)
    (else
      (bind _returnvalue_11 (Game|SpawnActorfromClass "/Game/Items/PickUp/SecretHelper/BP_EndingRune.BP_EndingRune_C" (Math|Transform|MakeTransform (.location _returnvalue_5) (.rotation _returnvalue_5) "1.000000,1.000000,1.000000") "Undefined" "MultiplyWithRoot" 0 0))
      (Class|MortisSecretHelper|RegisterOwnedPickup _self_2 _returnvalue_11)
      (Class|MortisSecretHelperRunePickup|SetOwningSecretHelper _returnvalue_11 _self_2))))

(event Collision|EventActorBeginOverlap
  (params (OtherActor :type Actor%20Object%20Reference)))

(event EventTick
  (params (DeltaSeconds :type Float%20%28single-precision%29)))

(fn ConstructionScript)