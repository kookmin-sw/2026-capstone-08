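; BP_2ndFakeWallTrap is a one-shot ambush trap that opens a fake wall and spawns an enemy when the player enters its trigger box.
; The first overlap by BP_PlayerCharacter sets a Triggered flag, then hides and disables collision on every static mesh component tagged FakeWall within the actor.
; It then spawns a BP_RedGolem at the SpawnPoint component's world transform.
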(event OnComponentBeginOverlap(TriggerBox)
  (params (OverlappedComponent :type Primitive%20Component%20Object%20Reference) (OtherActor :type Actor%20Object%20Reference) (OtherComp :type Primitive%20Component%20Object%20Reference) (OtherBodyIndex :type Integer) (bFromSweep :type Boolean) (SweepResult :type Hit%20Result%20Structure%20%28by%20ref%29))
  (Utilities|Casting|CastToBP_PlayerCharacter OtherActor)
  (if (not (Variables|Default|GetbTriggered))
    (Variables|Default|SetbTriggered true)
    (for _array_element (Actor|GetComponentsbyTag "/Script/Engine.StaticMeshComponent" "FakeWall")
      (Development|SetHiddeninGame _array_element true false)
      (Collision|SetCollisionEnabled _array_element "NoCollision"))
    (Game|SpawnActorfromClass "/Game/Characters/Enemy/RedGolem/BP_RedGolem.BP_RedGolem_C" (Transformation|GetWorldTransform (Variables|Default|GetSpawnPoint)) "Undefined" "MultiplyWithRoot" 0 0)))

(event EventBeginPlay)

(event Collision|EventActorBeginOverlap
  (params (OtherActor :type Actor%20Object%20Reference)))

(event EventTick
  (params (DeltaSeconds :type Float%20%28single-precision%29)))

(fn ConstructionScript)