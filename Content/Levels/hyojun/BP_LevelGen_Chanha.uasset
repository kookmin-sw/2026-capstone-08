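; Procedural level generator that builds a dungeon floor of rooms and corridors at BeginPlay from the DataTable for the current concept.
; A queue grows the map from the start room along shuffled arrows, box-checking overlaps and hiding tag-matched walls.
; Reverse passes over spawned rooms fill missing treasure, store and combat rooms, then attach the boss room.
; Boss placement triggers enemy spawner registration and initialization with MortisSpawnSubsystem.
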(event EventBeginPlay
  (bind _returnvalue (Subsystems|GetMortisSpawnSubsystem))
  (bind _corridorroomclasses (Variables|Default|GetCorridorRoomClasses))
  (bind _combatroomclasses (Variables|Default|GetCombatRoomClasses))
  (bind _corridorroomclasses_2 (Variables|Default|GetCorridorRoomClasses))
  (bind _combatroomclasses_2 (Variables|Default|GetCombatRoomClasses))
  (bind _corridorroomclasses_3 (Variables|Default|GetCorridorRoomClasses))
  (bind _corridorroomclasses_4 (Variables|Default|GetCorridorRoomClasses))
  (bind _corridorroomclasses_5 (Variables|Default|GetCorridorRoomClasses))
  ;[0.15 0.15 0.15 0.5] 데이터테이블을 이용한 각 층별 컨셉
  (bind _output_get (Variables|Default|SetCurrentRoomTable (Utilities|Select :Index (Variables|Default|GetCurrentConcept) :Option%200 (Variables|Default|GetDT_Level1) :Option%201 (Variables|Default|GetDT_Level2) :Option%202 (Variables|Default|GetDT_Level3))))
  (bind _outrownames (DataTable|GetDataTableRowNames _output_get))
  (for _array_element _outrownames
    (bind _returnvalue_2 (Utilities|GetDataTableRow (Variables|Default|GetCurrentRoomTable) _array_element)
      (:then
        (if (Utilities|Enum|Equal(Enum) (.RoomType (Utilities|Struct|BreakS_RoomData _returnvalue_2)) "NewEnumerator0")
          (Variables|Default|SetStartRoomClass (.RoomClass (Utilities|Struct|BreakS_RoomData _returnvalue_2)))
          (elif (Utilities|Enum|Equal(Enum) (.RoomType (Utilities|Struct|BreakS_RoomData _returnvalue_2)) "NewEnumerator1")
            (Utilities|Array|Add (Variables|Default|GetCombatRoomClasses) (.RoomClass (Utilities|Struct|BreakS_RoomData _returnvalue_2)))
            (elif (Utilities|Enum|Equal(Enum) (.RoomType (Utilities|Struct|BreakS_RoomData _returnvalue_2)) "NewEnumerator5")
              (Utilities|Array|Add (Variables|Default|GetCorridorRoomClasses) (.RoomClass (Utilities|Struct|BreakS_RoomData _returnvalue_2)))
              (elif (Utilities|Enum|Equal(Enum) (.RoomType (Utilities|Struct|BreakS_RoomData _returnvalue_2)) "NewEnumerator2")
                (Variables|Default|SetBossRoomClass (.RoomClass (Utilities|Struct|BreakS_RoomData _returnvalue_2)))
                (elif (Utilities|Enum|Equal(Enum) (.RoomType (Utilities|Struct|BreakS_RoomData _returnvalue_2)) "NewEnumerator3")
                  (Variables|Default|SetTreasureRoomClass (.RoomClass (Utilities|Struct|BreakS_RoomData _returnvalue_2)))
                  (elif (Utilities|Enum|Equal(Enum) (.RoomType (Utilities|Struct|BreakS_RoomData _returnvalue_2)) "NewEnumerator4")
                    (Variables|Default|SetBonusRoomClass (.RoomClass (Utilities|Struct|BreakS_RoomData _returnvalue_2)))
                    (elif (Utilities|Enum|Equal(Enum) (.RoomType (Utilities|Struct|BreakS_RoomData _returnvalue_2)) "NewEnumerator6")
                      (Variables|Default|SetStoreRoomClass (.RoomClass (Utilities|Struct|BreakS_RoomData _returnvalue_2)))
                      (elif (Utilities|Enum|Equal(Enum) (.RoomType (Utilities|Struct|BreakS_RoomData _returnvalue_2)) "NewEnumerator7")
                        (Variables|Default|SetStairRoomClass (.RoomClass (Utilities|Struct|BreakS_RoomData _returnvalue_2))))))))))))))
  ;[0.15 0.15 0.15 0.5] 첫번째 방 생성 및 첫번째 방의 화살표 정보 저장
  (bind _returnvalue_3 (Game|SpawnActorfromClass (Variables|Default|GetStartRoomClass) (Math|Transform|MakeTransform "0, 0, 0") "Undefined" "MultiplyWithRoot" 0 0))
  (Variables|Default|SetNextRoomList (Utilities|Array|MakeArray _returnvalue_3))
  ;[0.15 0.15 0.15 0.5] 다음에 나올 방이 있고, 만든 방 개수가 목표 이하면 계속 방만들기
  (while (and (> (Utilities|Array|Length (Variables|Default|GetNextRoomList)) 0) (< (Variables|Default|GetRoomCount) (Variables|Default|GetMaxCount)))
    ;[0.15 0.15 0.15 0.5] 다음으로 만들 방 확인 및 중복생성 방지를 위한 제거
    (bind _output_get_2 (Variables|Default|SetProcessing%20Room (Utilities|Array|Get(acopy) (Variables|Default|GetNextRoomList))))
    (Utilities|Array|RemoveIndex (Variables|Default|GetNextRoomList))
    ;[0.15 0.15 0.15 0.5] 단조로운 맵 생성 방지를 위해 3방향중 랜덤개수만큼 랜덤 방향으로 설정
    (bind _output_get_3 (Variables|Default|SetRandomRoom (Actor|GetComponentsByClass _output_get_2 "/Script/Engine.ArrowComponent")))
    (Utilities|Array|Shuffle _output_get_3)
    (bind _output_get_4 (Variables|Default|SetRandomCount (.OutItem (Utilities|Array|Random (Utilities|Array|MakeArray 1 1 2 2 2 3 3)))))
    ;[0.15 0.15 0.15 0.5] 지정된 개수, 방향으로 각각 방 생성
    (for (_array_element_2 _array_index) (Variables|Default|GetRandomRoom)
      ;[0.15 0.15 0.15 0.5] 검사
      (if (< _array_index _output_get_4)
        (Utilities|IsValid (Utilities|Array|Get(acopy) (Actor|GetComponentsbyTag (Variables|Default|GetProcessing%20Room) "/Script/Engine.StaticMeshComponent" (Utilities|Array|Get(acopy) (Variables|/Script/Engine.ActorComponent|GetComponentTags _array_element_2))))
          (:Is%20Valid
            ;[0.15 0.15 0.15 0.5] 충돌 검사
            (bind _returnvalue_4 (Collision|BoxOverlapActors (+ (.Location (Math|Transform|BreakTransform (Transformation|GetWorldTransform _array_element_2))) (* (Math|Vector|GetForwardVector (.Rotation (Math|Transform|BreakTransform (Transformation|GetWorldTransform _array_element_2)))) 3000)) "1200.000000,1200.000000,0.000000" (Utilities|Array|MakeArray "ObjectTypeQuery1" "ObjectTypeQuery2") 0 :!class /Script/Engine.KismetSystemLibrary))
            (if (not _returnvalue_4)
              ;[0.15 0.15 0.15 0.5] 만약 충돌이 없고 방을 만들 예정이라면 막고있던 벽 지우기
              (for _array_element_3 (Actor|GetComponentsbyTag (Variables|Default|GetProcessing%20Room) "/Script/Engine.StaticMeshComponent" (Utilities|Array|Get(acopy) (Variables|/Script/Engine.ActorComponent|GetComponentTags _array_element_2)))
                (Development|SetHiddeninGame _array_element_3 true true)
                (Collision|SetCollisionEnabled _array_element_3 "NoCollision"))
              ;[0.15 0.15 0.15 0.5] 터널 생성 후 위치정보 갱신
              (bind _returnvalue_5 (Game|SpawnActorfromClass (Utilities|Array|Get(acopy) _corridorroomclasses_3 (Math|Random|RandomIntegerinRange 0 (- (Utilities|Array|Length _corridorroomclasses_3) 1))) (Transformation|GetWorldTransform _array_element_2) "Undefined" "MultiplyWithRoot" 0 0))
              (Variables|/Game/Levels/hyojun/BP_RoomBase.BP_RoomBase_C|SetRoomType _returnvalue_5 "NewEnumerator5")
              (if (< (Math|Random|RandomFloatinRange 0.0 1.0) 0.2)
                (if (< (Variables|Default|GetSpawnedTreasureCount) 1)
                  (bind _returnvalue_6 (Game|SpawnActorfromClass (Variables|Default|GetTreasureRoomClass) (Transformation|GetWorldTransform (Variables|/Game/Levels/hyojun/BP_RoomBase.BP_RoomBase_C|GetExitPoint _returnvalue_5)) "Undefined" "MultiplyWithRoot" 0 0))
                  (Variables|/Game/Levels/hyojun/BP_RoomBase.BP_RoomBase_C|SetRoomType _returnvalue_6 "NewEnumerator3")
                  (Math|Integer|IncrementInt (Variables|Default|GetRoomCount)
                    (:%20%20
                      (Utilities|Array|Add (Variables|Default|GetNextRoomList) _returnvalue_6)
                      (Utilities|Array|Add (Variables|Default|GetSpawnedRooms) _returnvalue_6)
                      (Math|Integer|IncrementInt (Variables|Default|GetSpawnedTreasureCount)
                        (:%20%20
                          (Utilities|Array|Add (Variables|/Game/Levels/hyojun/BP_RoomBase.BP_RoomBase_C|GetConnectedRooms (Variables|Default|GetProcessing%20Room)) _returnvalue_6)
                          (Utilities|Array|Add (Variables|/Game/Levels/hyojun/BP_RoomBase.BP_RoomBase_C|GetConnectedRooms _returnvalue_6) _returnvalue_6)))))
                  (elif (< (Variables|Default|GetSpawnedStoreCount) 1)
                    (bind _returnvalue_7 (Game|SpawnActorfromClass (Variables|Default|GetStoreRoomClass) (Transformation|GetWorldTransform (Variables|/Game/Levels/hyojun/BP_RoomBase.BP_RoomBase_C|GetExitPoint _returnvalue_5)) "Undefined" "MultiplyWithRoot" 0 0))
                    (Variables|/Game/Levels/hyojun/BP_RoomBase.BP_RoomBase_C|SetRoomType _returnvalue_7 "NewEnumerator6")
                    (Math|Integer|IncrementInt (Variables|Default|GetRoomCount)
                      (:%20%20
                        (Utilities|Array|Add (Variables|Default|GetNextRoomList) _returnvalue_7)
                        (Utilities|Array|Add (Variables|Default|GetSpawnedRooms) _returnvalue_7)
                        (Math|Integer|IncrementInt (Variables|Default|GetSpawnedStoreCount)
                          (:%20%20
                            (Utilities|Array|Add (Variables|/Game/Levels/hyojun/BP_RoomBase.BP_RoomBase_C|GetConnectedRooms (Variables|Default|GetProcessing%20Room)) _returnvalue_7)
                            (Utilities|Array|Add (Variables|/Game/Levels/hyojun/BP_RoomBase.BP_RoomBase_C|GetConnectedRooms _returnvalue_7) _returnvalue_7)))))
                    (elif (< (Variables|Default|GetCurrentBonusCount) (Variables|Default|GetMaxBonusCount))
                      (bind _returnvalue_8 (Game|SpawnActorfromClass (Variables|Default|GetBonusRoomClass) (Transformation|GetWorldTransform (Variables|/Game/Levels/hyojun/BP_RoomBase.BP_RoomBase_C|GetExitPoint _returnvalue_5)) "Undefined" "MultiplyWithRoot" 0 0))
                      (Variables|/Game/Levels/hyojun/BP_RoomBase.BP_RoomBase_C|SetRoomType _returnvalue_8 "NewEnumerator4")
                      (Math|Integer|IncrementInt (Variables|Default|GetRoomCount)
                        (:%20%20
                          (Utilities|Array|Add (Variables|Default|GetNextRoomList) _returnvalue_8)
                          (Utilities|Array|Add (Variables|Default|GetSpawnedRooms) _returnvalue_8)
                          (Math|Integer|IncrementInt (Variables|Default|GetCurrentBonusCount)
                            (:%20%20
                              (Utilities|Array|Add (Variables|/Game/Levels/hyojun/BP_RoomBase.BP_RoomBase_C|GetConnectedRooms (Variables|Default|GetProcessing%20Room)) _returnvalue_8)
                              (Utilities|Array|Add (Variables|/Game/Levels/hyojun/BP_RoomBase.BP_RoomBase_C|GetConnectedRooms _returnvalue_8) _returnvalue_8)))))
                      (else
                        ;[0.15 0.15 0.15 0.5] 일반방 스폰
                        (bind _returnvalue_9 (Game|SpawnActorfromClass (Utilities|Array|Get(acopy) _combatroomclasses (Math|Random|RandomIntegerinRange 0 (- (Utilities|Array|Length _combatroomclasses) 1))) (Transformation|GetWorldTransform (Variables|/Game/Levels/hyojun/BP_RoomBase.BP_RoomBase_C|GetExitPoint _returnvalue_5)) "AlwaysSpawn" "MultiplyWithRoot" 0 0 :!label _label))
                        (Variables|/Game/Levels/hyojun/BP_RoomBase.BP_RoomBase_C|SetRoomType _returnvalue_9 "NewEnumerator1")
                        ;[0.15 0.15 0.15 0.5] 방 개수 카운트 증가 및 만들 방 정보 갱신 후 전체 방 정보 저장
                        (Math|Integer|IncrementInt (Variables|Default|GetRoomCount)
                          (:%20%20
                            (Utilities|Array|Add (Variables|Default|GetNextRoomList) _returnvalue_9)
                            (Utilities|Array|Add (Variables|Default|GetSpawnedRooms) _returnvalue_9)
                            (Utilities|Array|Add (Variables|/Game/Levels/hyojun/BP_RoomBase.BP_RoomBase_C|GetConnectedRooms (Variables|Default|GetProcessing%20Room)) _returnvalue_9)
                            (Utilities|Array|Add (Variables|/Game/Levels/hyojun/BP_RoomBase.BP_RoomBase_C|GetConnectedRooms _returnvalue_9) _returnvalue_9)))))))
                (else
                  (goto _label)))))))))
  (while (< (Variables|Default|GetSpawnedTreasureCount) 1)
    ;[0.15 0.15 0.15 0.5] 마지막 생성 방부터 하나씩 위치정보 가져오기 방 개수 다 채울때까지 반복
    (bind _arrayelement (Utilities|Array|ReverseforEachLoop (Variables|Default|GetSpawnedRooms))
      (:LoopBody
        (if (< (Variables|Default|GetSpawnedTreasureCount) 1)
          (for _array_element_4 (Actor|GetComponentsByClass _arrayelement "/Script/Engine.ArrowComponent")
            (if (< (Variables|Default|GetSpawnedTreasureCount) 1)
              ;[0.15 0.15 0.15 0.5] 방 생성 전 충돌검사
              (bind _returnvalue_10 (Collision|BoxOverlapActors (+ (.Location (Math|Transform|BreakTransform (Transformation|GetWorldTransform _array_element_4))) (* (Math|Vector|GetForwardVector (.Rotation (Math|Transform|BreakTransform (Transformation|GetWorldTransform _array_element_4)))) 2400)) "1500.000000,1500.000000,0.000000" (Utilities|Array|MakeArray "ObjectTypeQuery1" "ObjectTypeQuery2") 0 :!class /Script/Engine.KismetSystemLibrary))
              (if (not _returnvalue_10)
                ;[0.15 0.15 0.15 0.5] 해당 방향에 있는 문 제거
                (for _array_element_5 (Actor|GetComponentsbyTag _arrayelement "/Script/Engine.StaticMeshComponent" (Utilities|Array|Get(acopy) (Variables|/Script/Engine.ActorComponent|GetComponentTags _array_element_4)))
                  (Development|SetHiddeninGame _array_element_5 true true)
                  (Collision|SetCollisionEnabled _array_element_5 "NoCollision"))
                ;[0.15 0.15 0.15 0.5] 충돌이 없다면 생성
                (bind _returnvalue_11 (Game|SpawnActorfromClass (Utilities|Array|Get(acopy) _corridorroomclasses_4 (Math|Random|RandomIntegerinRange 0 (- (Utilities|Array|Length _corridorroomclasses_4) 1))) (Transformation|GetWorldTransform _array_element_4) "Undefined" "MultiplyWithRoot" 0 0))
                (Variables|/Game/Levels/hyojun/BP_RoomBase.BP_RoomBase_C|SetRoomType _returnvalue_11 "NewEnumerator5")
                (bind _returnvalue_12 (Game|SpawnActorfromClass (Variables|Default|GetTreasureRoomClass) (Transformation|GetWorldTransform (Utilities|Array|Get(acopy) (Actor|GetComponentsByClass _returnvalue_11 "/Script/Engine.ArrowComponent"))) "Undefined" "MultiplyWithRoot" 0 0))
                (Variables|/Game/Levels/hyojun/BP_RoomBase.BP_RoomBase_C|SetRoomType _returnvalue_12 "NewEnumerator3")
                (Utilities|Array|Add (Variables|Default|GetSpawnedRooms) _returnvalue_12)
                (Math|Integer|IncrementInt (Variables|Default|GetRoomCount)
                  (:%20%20
                    (Math|Integer|IncrementInt (Variables|Default|GetSpawnedTreasureCount)
                      (:%20%20
                        (Utilities|Array|Add (Variables|/Game/Levels/hyojun/BP_RoomBase.BP_RoomBase_C|GetConnectedRooms (Variables|Default|GetProcessing%20Room)) _returnvalue_12)
                        (Utilities|Array|Add (Variables|/Game/Levels/hyojun/BP_RoomBase.BP_RoomBase_C|GetConnectedRooms _returnvalue_12) _returnvalue_12))))))))))))
  (while (< (Variables|Default|GetSpawnedStoreCount) 1)
    ;[0.15 0.15 0.15 0.5] 마지막 생성 방부터 하나씩 위치정보 가져오기 방 개수 다 채울때까지 반복
    (bind _arrayelement_2 (Utilities|Array|ReverseforEachLoop (Variables|Default|GetSpawnedRooms))
      (:LoopBody
        (if (< (Variables|Default|GetSpawnedStoreCount) 1)
          (for _array_element_6 (Actor|GetComponentsByClass _arrayelement_2 "/Script/Engine.ArrowComponent")
            (if (< (Variables|Default|GetSpawnedStoreCount) 1)
              ;[0.15 0.15 0.15 0.5] 방 생성 전 충돌검사
              (bind _returnvalue_13 (Collision|BoxOverlapActors (+ (.Location (Math|Transform|BreakTransform (Transformation|GetWorldTransform _array_element_6))) (* (Math|Vector|GetForwardVector (.Rotation (Math|Transform|BreakTransform (Transformation|GetWorldTransform _array_element_6)))) 3600)) "1500.000000,1500.000000,0.000000" (Utilities|Array|MakeArray "ObjectTypeQuery1" "ObjectTypeQuery2") 0 :!class /Script/Engine.KismetSystemLibrary))
              (if (not _returnvalue_13)
                ;[0.15 0.15 0.15 0.5] 해당 방향에 있는 문 제거
                (for _array_element_7 (Actor|GetComponentsbyTag _arrayelement_2 "/Script/Engine.StaticMeshComponent" (Utilities|Array|Get(acopy) (Variables|/Script/Engine.ActorComponent|GetComponentTags _array_element_6)))
                  (Development|SetHiddeninGame _array_element_7 true true)
                  (Collision|SetCollisionEnabled _array_element_7 "NoCollision"))
                ;[0.15 0.15 0.15 0.5] 충돌이 없다면 생성
                (bind _returnvalue_14 (Game|SpawnActorfromClass (Utilities|Array|Get(acopy) _corridorroomclasses (Math|Random|RandomIntegerinRange 0 (- (Utilities|Array|Length _corridorroomclasses) 1))) (Transformation|GetWorldTransform _array_element_6) "Undefined" "MultiplyWithRoot" 0 0))
                (Variables|/Game/Levels/hyojun/BP_RoomBase.BP_RoomBase_C|SetRoomType _returnvalue_14 "NewEnumerator5")
                (bind _returnvalue_15 (Game|SpawnActorfromClass (Variables|Default|GetStoreRoomClass) (Transformation|GetWorldTransform (Utilities|Array|Get(acopy) (Actor|GetComponentsByClass _returnvalue_14 "/Script/Engine.ArrowComponent"))) "Undefined" "MultiplyWithRoot" 0 0))
                (Variables|/Game/Levels/hyojun/BP_RoomBase.BP_RoomBase_C|SetRoomType _returnvalue_15 "NewEnumerator6")
                (Utilities|Array|Add (Variables|Default|GetSpawnedRooms) _returnvalue_15)
                (Math|Integer|IncrementInt (Variables|Default|GetRoomCount)
                  (:%20%20
                    (Math|Integer|IncrementInt (Variables|Default|GetSpawnedStoreCount)
                      (:%20%20
                        (Utilities|Array|Add (Variables|/Game/Levels/hyojun/BP_RoomBase.BP_RoomBase_C|GetConnectedRooms (Variables|Default|GetProcessing%20Room)) _returnvalue_15)
                        (Utilities|Array|Add (Variables|/Game/Levels/hyojun/BP_RoomBase.BP_RoomBase_C|GetConnectedRooms _returnvalue_15) _returnvalue_15))))))))))))
  (while (< (Variables|Default|GetRoomCount) (Variables|Default|GetMaxCount))
    ;[0.15 0.15 0.15 0.5] 마지막 생성 방부터 하나씩 위치정보 가져오기 방 개수 다 채울때까지 반복
    (bind _arrayelement_3 (Utilities|Array|ReverseforEachLoop (Variables|Default|GetSpawnedRooms))
      (:LoopBody
        (if (< (Variables|Default|GetRoomCount) (Variables|Default|GetMaxCount))
          (for _array_element_8 (Actor|GetComponentsByClass _arrayelement_3 "/Script/Engine.ArrowComponent")
            (if (< (Variables|Default|GetRoomCount) (Variables|Default|GetMaxCount))
              ;[0.15 0.15 0.15 0.5] 방 생성 전 충돌검사
              (bind _returnvalue_16 (Collision|BoxOverlapActors (+ (.Location (Math|Transform|BreakTransform (Transformation|GetWorldTransform _array_element_8))) (* (Math|Vector|GetForwardVector (.Rotation (Math|Transform|BreakTransform (Transformation|GetWorldTransform _array_element_8)))) 3600)) "1500.000000,1500.000000,0.000000" (Utilities|Array|MakeArray "ObjectTypeQuery1" "ObjectTypeQuery2") 0 :!class /Script/Engine.KismetSystemLibrary))
              (if (not _returnvalue_16)
                ;[0.15 0.15 0.15 0.5] 해당 방향에 있는 문 제거
                (for _array_element_9 (Actor|GetComponentsbyTag _arrayelement_3 "/Script/Engine.StaticMeshComponent" (Utilities|Array|Get(acopy) (Variables|/Script/Engine.ActorComponent|GetComponentTags _array_element_8)))
                  (Development|SetHiddeninGame _array_element_9 true true)
                  (Collision|SetCollisionEnabled _array_element_9 "NoCollision"))
                ;[0.15 0.15 0.15 0.5] 충돌이 없다면 생성
                (bind _returnvalue_17 (Game|SpawnActorfromClass (Utilities|Array|Get(acopy) _corridorroomclasses_5 (Math|Random|RandomIntegerinRange 0 (- (Utilities|Array|Length _corridorroomclasses_5) 1))) (Transformation|GetWorldTransform _array_element_8) "Undefined" "MultiplyWithRoot" 0 0))
                (Variables|/Game/Levels/hyojun/BP_RoomBase.BP_RoomBase_C|SetRoomType _returnvalue_17 "NewEnumerator5")
                (bind _returnvalue_18 (Game|SpawnActorfromClass (Utilities|Array|Get(acopy) _combatroomclasses_2 (Math|Random|RandomIntegerinRange 0 (- (Utilities|Array|Length _combatroomclasses_2) 1))) (Transformation|GetWorldTransform (Utilities|Array|Get(acopy) (Actor|GetComponentsByClass _returnvalue_17 "/Script/Engine.ArrowComponent"))) "Undefined" "MultiplyWithRoot" 0 0))
                (Variables|/Game/Levels/hyojun/BP_RoomBase.BP_RoomBase_C|SetRoomType _returnvalue_18 "NewEnumerator1")
                (Utilities|Array|Add (Variables|Default|GetSpawnedRooms) _returnvalue_18)
                (Math|Integer|IncrementInt (Variables|Default|GetRoomCount)
                  (:%20%20
                    (Utilities|Array|Add (Variables|/Game/Levels/hyojun/BP_RoomBase.BP_RoomBase_C|GetConnectedRooms (Variables|Default|GetProcessing%20Room)) _returnvalue_18)
                    (Utilities|Array|Add (Variables|/Game/Levels/hyojun/BP_RoomBase.BP_RoomBase_C|GetConnectedRooms _returnvalue_18) _returnvalue_18))))))))))
  ;[0.15 0.15 0.15 0.5] 마지막 생성 방부터 하나씩 위치정보 가져오기, 보스 방 만들때까지 반복
  (Variables|Default|SetIsBossSpawned false)
  (bind _arrayelement_4 (Utilities|Array|ReverseforEachLoop (Variables|Default|GetSpawnedRooms))
    (:LoopBody
      (if (not (Variables|Default|GetIsBossSpawned))
        ;[0.15 0.15 0.15 0.5] 보스방, 계단방 생성 전 충돌검사
        (bind _returnvalue_19 (Collision|BoxOverlapActors (+ (.Location (Math|Transform|BreakTransform (Transformation|GetWorldTransform (Utilities|Array|Get(acopy) (Actor|GetComponentsByClass _arrayelement_4 "/Script/Engine.ArrowComponent"))))) (* (Math|Vector|GetForwardVector (.Rotation (Math|Transform|BreakTransform (Transformation|GetWorldTransform (Utilities|Array|Get(acopy) (Actor|GetComponentsByClass _arrayelement_4 "/Script/Engine.ArrowComponent")))))) 3600)) "1500.000000,1500.000000,0.000000" (Utilities|Array|MakeArray "ObjectTypeQuery1" "ObjectTypeQuery2") 0 :!class /Script/Engine.KismetSystemLibrary))
        (if (not _returnvalue_19)
          (if (not (Variables|Default|GetIsBossSpawned))
            ;[0.15 0.15 0.15 0.5] 보스 방 생성시 해당 방향에 있는 문 제거
            (for _array_element_10 (Actor|GetComponentsbyTag _arrayelement_4 "/Script/Engine.StaticMeshComponent" (Utilities|Array|Get(acopy) (Variables|/Script/Engine.ActorComponent|GetComponentTags (Utilities|Array|Get(acopy) (Actor|GetComponentsByClass _arrayelement_4 "/Script/Engine.ArrowComponent")))))
              (Development|SetHiddeninGame _array_element_10 true true)
              (Collision|SetCollisionEnabled _array_element_10 "NoCollision"))
            (if (not (Variables|Default|GetIsBossSpawned))
              ;[0.15 0.15 0.15 0.5] 충돌이 없다면 통로 및 보스방 혹은 계단방 생성
              (bind _returnvalue_20 (Game|SpawnActorfromClass (Utilities|Array|Get(acopy) _corridorroomclasses_2 (Math|Random|RandomIntegerinRange 0 (- (Utilities|Array|Length _corridorroomclasses_2) 1))) (Transformation|GetWorldTransform (Utilities|Array|Get(acopy) (Actor|GetComponentsByClass _arrayelement_4 "/Script/Engine.ArrowComponent"))) "Undefined" "MultiplyWithRoot" 0 0))
              (Variables|/Game/Levels/hyojun/BP_RoomBase.BP_RoomBase_C|SetRoomType _returnvalue_20 "NewEnumerator5")
              (bind _returnvalue_21 (Game|SpawnActorfromClass (Variables|Default|GetBossRoomClass) (Transformation|GetWorldTransform (Utilities|Array|Get(acopy) (Actor|GetComponentsByClass _returnvalue_20 "/Script/Engine.ArrowComponent"))) "Undefined" "MultiplyWithRoot" 0 0))
              (Variables|Default|SetIsBossSpawned true)
              (Utilities|Array|Add (Variables|Default|GetSpawnedRooms) _returnvalue_21)
              (Variables|/Game/Levels/hyojun/BP_RoomBase.BP_RoomBase_C|SetRoomType _returnvalue_21 "NewEnumerator2")
              (Utilities|Array|Add (Variables|/Game/Levels/hyojun/BP_RoomBase.BP_RoomBase_C|GetConnectedRooms (Variables|Default|GetProcessing%20Room)) _returnvalue_21)
              (Utilities|Array|Add (Variables|/Game/Levels/hyojun/BP_RoomBase.BP_RoomBase_C|GetConnectedRooms _returnvalue_21) _returnvalue_21)
              (for _array_element_11 (Variables|Default|GetSpawnedRooms)
                (Default|SetEnemySpawner _array_element_11)
                (Class|MortisSpawnSubsystem|RegisterSpawner _returnvalue (Variables|/Game/Levels/hyojun/BP_RoomBase.BP_RoomBase_C|GetBP_EnemySpawnerComponent _array_element_11)))
              (Class|MortisSpawnSubsystem|InitializeSpawnPoints _returnvalue))))))))

(event Collision|EventActorBeginOverlap
  (params (OtherActor :type Actor%20Object%20Reference)))

(event EventTick
  (params (DeltaSeconds :type Float%20%28single-precision%29)))

(fn ConstructionScript)