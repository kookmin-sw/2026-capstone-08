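; Room base actor that handles enemy spawning, door lockdown and clear state for a level of connected rooms.
; Player overlap marks the room visited and triggers spawning in it and its ConnectedRooms, so neighbors populate ahead of entry.
; One room type reveals "Door"-tagged meshes as barriers, reopened once all spawned enemies are destroyed; the other combat type's random lock chance is zero.
; ResetRoom clears state and destroys remaining enemies.
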(event OnComponentBeginOverlap(Box)
  (params (OverlappedComponent :type Primitive%20Component%20Object%20Reference) (OtherActor :type Actor%20Object%20Reference) (OtherComp :type Primitive%20Component%20Object%20Reference) (OtherBodyIndex :type Integer) (bFromSweep :type Boolean) (SweepResult :type Hit%20Result%20Structure%20%28by%20ref%29))
  (Utilities|Casting|CastToBP_PlayerCharacter OtherActor)
  (Variables|Default|SetbVisited true)
  (CallFunction|SpawnEnemiesbySpanwer)
  (for _array_element (Variables|Default|GetConnectedRooms)
    (CallFunction|SpawnEnemiesbySpanwer _array_element))
  (if (or (Utilities|Enum|Equal(Enum) (Variables|Default|GetRoomType) "NewEnumerator1") (Utilities|Enum|Equal(Enum) (Variables|Default|GetRoomType) "NewEnumerator2"))
    (if (not (Variables|Default|GetbRoomCleared))
      (if (Utilities|Enum|Equal(Enum) (Variables|Default|GetRoomType) "NewEnumerator2")
        (for _array_element_2 (Actor|GetComponentsbyTag "/Script/Engine.StaticMeshComponent" "Door") :!label _label
          (if (not (Rendering|IsVisible _array_element_2))
            (Collision|SetCollisionEnabled _array_element_2 "QueryAndPhysics")
            (Development|SetHiddeninGame _array_element_2 false true)
            (Utilities|Array|Add (Variables|Default|GetLockedDoors) _array_element_2)))
        (elif (< (Math|Random|RandomFloatinRange 0.0 1.0) 0.0)
          (goto _label))))))

(event Custom|OnEnemyDestroyed
  (params (DestroyedActor :type Actor%20Object%20Reference))
  (Utilities|Array|RemoveItem (Variables|Default|GetSpawnedEnemies) DestroyedActor)
  (if (Utilities|Array|IsEmpty (Variables|Default|GetSpawnedEnemies))
    (for _array_element (Variables|Default|GetLockedDoors)
      (Collision|SetCollisionEnabled _array_element "NoCollision")
      (Development|SetHiddeninGame _array_element true false)
      (Variables|Default|SetbRoomCleared true))))

(event Custom|SpawnEnemiesBySpanwer
  (if (or (and (Utilities|Enum|Equal(Enum) (Variables|Default|GetRoomType) "NewEnumerator2") (Utilities|Array|IsEmpty (Variables|Default|GetSpawnedEnemies))) (not (Variables|Default|GetbRoomActivated)))
    (Variables|Default|SetbRoomActivated true)
    (if (or (Utilities|Enum|Equal(Enum) (Variables|Default|GetRoomType) "NewEnumerator1") (Utilities|Enum|Equal(Enum) (Variables|Default|GetRoomType) "NewEnumerator2"))
      (bind _returnvalue (Class|MortisEnemySpawnerComponent|SpawnEnemies (Variables|Default|GetBP_EnemySpawnerComponent)))
      (bind _output_get (Variables|Default|SetSpawnedEnemies _returnvalue))
      (if (Utilities|Array|IsEmpty _output_get)
        (for _array_element (Variables|Default|GetLockedDoors)
          (Collision|SetCollisionEnabled _array_element "NoCollision")
          (Development|SetHiddeninGame _array_element true false)
          (Variables|Default|SetbRoomCleared true))
        (else
          (for _array_element_2 (Variables|Default|GetSpawnedEnemies)
            (Game|BindEventtoOnDestroyed _array_element_2 (delegate Custom|OnEnemyDestroyed))))))))

(event Collision|EventActorBeginOverlap
  (params (OtherActor :type Actor%20Object%20Reference)))

(event EventTick
  (params (DeltaSeconds :type Float%20%28single-precision%29)))

(fn ConstructionScript)

(fn ResetRoom
  (Variables|Default|SetbRoomActivated false)
  (Variables|Default|SetbRoomCleared false)
  (Variables|Default|SetbVisited false)
  (CallFunction|DestroySpawnedEnemies))

(fn DestroySpawnedEnemies
  (for _array_element (Variables|Default|GetSpawnedEnemies)
    (EventDispatchers|UnbindallEventsfromOnDestroyed _array_element)
    (Actor|DestroyActor _array_element))
  (Utilities|Array|Clear (Variables|Default|GetSpawnedEnemies)))