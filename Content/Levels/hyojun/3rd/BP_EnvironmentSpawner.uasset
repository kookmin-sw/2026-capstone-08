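; Environment spawner that randomly scatters vegetation, trees and ruins across the level once, shortly after BeginPlay.
; Each iteration line-traces between random high and low points within SpawnRadius of world origin, skipping hits tagged Room or near a BP_RoomBase.
; A cascade of random rolls picks the HISM component that receives an instance at the impact point.
; Ruins get random yaw and a wider room clearance, falling back to a tree when too close.
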(event Custom|SpawnEnvironment)

(event EventBeginPlay
  (bind _returnvalue (Math|Random|RandomFloatinRange 0.0 1.0))
  (Utilities|FlowControl|Delay 1.0)
  (for _index (range 0 (Variables|Default|GetSpawnCount))
    (bind (_outhit _returnvalue_2) (Collision|LineTraceByChannel (Math|Vector|MakeVector (Math|Random|RandomFloatinRange (Math|Conversions|ToFloat(Integer) (* (Variables|Default|GetSpawnRadius) -1)) (Math|Conversions|ToFloat(Integer) (Variables|Default|GetSpawnRadius))) (Math|Random|RandomFloatinRange (Math|Conversions|ToFloat(Integer) (* (Variables|Default|GetSpawnRadius) -1)) (Math|Conversions|ToFloat(Integer) (Variables|Default|GetSpawnRadius))) 5e+03) (Math|Vector|MakeVector (Math|Random|RandomFloatinRange (Math|Conversions|ToFloat(Integer) (* (Variables|Default|GetSpawnRadius) -1)) (Math|Conversions|ToFloat(Integer) (Variables|Default|GetSpawnRadius))) (Math|Random|RandomFloatinRange (Math|Conversions|ToFloat(Integer) (* (Variables|Default|GetSpawnRadius) -1)) (Math|Conversions|ToFloat(Integer) (Variables|Default|GetSpawnRadius))) -5e+03) "TraceTypeQuery1" false 0 "None"))
    (if (not (Actor|ActorHasTag (.HitActor (Collision|BreakHitResult _outhit)) "Room"))
      (bind _outactors (Collision|SphereOverlapActors (.ImpactPoint (Collision|BreakHitResult _outhit)) 3e+02 (Utilities|Array|MakeArray "ObjectTypeQuery2") "/Game/Levels/hyojun/BP_RoomBase.BP_RoomBase_C"))
      (if (not (> (Utilities|Array|Length _outactors) 0))
        (if _returnvalue_2
          (if (< _returnvalue 0.05)
            (Components|InstancedStaticMesh|AddInstance (Variables|Default|GetHISM_Weed) (Math|Conversions|ToTransform(Vector) (.ImpactPoint (Collision|BreakHitResult _outhit))) true)
            (elif (< _returnvalue 0.1)
              (Components|InstancedStaticMesh|AddInstance (Variables|Default|GetHISM_Bush) (Math|Conversions|ToTransform(Vector) (.ImpactPoint (Collision|BreakHitResult _outhit))) true)
              (elif (< _returnvalue 0.3)
                (Components|InstancedStaticMesh|AddInstance (Variables|Default|GetHISM_Pine) (Math|Conversions|ToTransform(Vector) (.ImpactPoint (Collision|BreakHitResult _outhit))) true)
                (elif (< _returnvalue 0.5)
                  (Components|InstancedStaticMesh|AddInstance (Variables|Default|GetHISM_DeadTree) (Math|Conversions|ToTransform(Vector) (.ImpactPoint (Collision|BreakHitResult _outhit))) true)
                  (elif (< _returnvalue 0.7)
                    (Components|InstancedStaticMesh|AddInstance (Variables|Default|GetHISM_Tree) (Math|Conversions|ToTransform(Vector) (.ImpactPoint (Collision|BreakHitResult _outhit))) true :!label _label)
                    (else
                      (bind _outactors_2 (Collision|SphereOverlapActors (.ImpactPoint (Collision|BreakHitResult _outhit)) 1.5e+03 (Utilities|Array|MakeArray "ObjectTypeQuery2") "/Game/Levels/hyojun/BP_RoomBase.BP_RoomBase_C"))
                      (if (> (Utilities|Array|Length _outactors_2) 0)
                        (goto _label)
                        (elif (< _returnvalue 0.8)
                          (Components|InstancedStaticMesh|AddInstance (Variables|Default|GetHISM_Ruin) (Math|Transform|MakeTransform (.ImpactPoint (Collision|BreakHitResult _outhit)) (Math|Rotator|MakeRotator 0.0 0.0 (Math|Random|RandomFloatinRange 0.0 3.6e+02))) true)
                          (elif (< _returnvalue 0.9)
                            (Components|InstancedStaticMesh|AddInstance (Variables|Default|GetHISM_Ruin1) (Math|Transform|MakeTransform (.ImpactPoint (Collision|BreakHitResult _outhit)) (Math|Rotator|MakeRotator 0.0 0.0 (Math|Random|RandomFloatinRange 0.0 3.6e+02))) true)
                            (else
                              (Components|InstancedStaticMesh|AddInstance (Variables|Default|GetHISM_Ruin2) (Math|Transform|MakeTransform (.ImpactPoint (Collision|BreakHitResult _outhit)) (Math|Rotator|MakeRotator 0.0 0.0 (Math|Random|RandomFloatinRange 0.0 3.6e+02))) true))))))))))))))))

(event Collision|EventActorBeginOverlap
  (params (OtherActor :type Actor%20Object%20Reference)))

(event EventTick
  (params (DeltaSeconds :type Float%20%28single-precision%29)))

(fn ConstructionScript)