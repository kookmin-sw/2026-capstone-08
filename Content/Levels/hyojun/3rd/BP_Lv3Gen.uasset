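; Procedural generator for the third level, building a dungeon of rooms and passages from a start room on BeginPlay.
; A queue expands rooms breadth-first until MaxCount, choosing shuffled arrow directions with a branch count weighted toward one.
; Box overlap checks reject blocked spots; otherwise tag-matched doors are disabled and a passage and cross room spawn.
; Finally, it attaches the boss room via a passage to the latest room whose first arrow is unobstructed.
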(event EventBeginPlay
  ;[0.15 0.15 0.15 0.5] 첫번째 방 생성 및 첫번째 방의 화살표 정보 저장
  (bind _returnvalue (Game|SpawnActorfromClass "/Game/Levels/hyojun/3rd/BP_3rdStart.BP_3rdStart_C" (Math|Transform|MakeTransform "0, 0, 0") "AlwaysSpawn" "MultiplyWithRoot" 0 0))
  (Variables|Default|SetNextRoomList (Utilities|Array|MakeArray _returnvalue))
  ;[0.15 0.15 0.15 0.5] 다음에 나올 방이 있고, 만든 방 개수가 목표 이하면 계속 방만들기
  (while (and (> (Utilities|Array|Length (Variables|Default|GetNextRoomList)) 0) (< (Variables|Default|GetRoomCount) (Variables|Default|GetMaxCount)))
    ;[0.15 0.15 0.15 0.5] 다음으로 만들 방 확인 및 중복생성 방지를 위한 제거
    (bind _output_get (Variables|Default|SetProcessing%20Room (Utilities|Array|Get(acopy) (Variables|Default|GetNextRoomList))))
    (Utilities|Array|RemoveIndex (Variables|Default|GetNextRoomList))
    ;[0.15 0.15 0.15 0.5] 단조로운 맵 생성 방지를 위해 3방향중 랜덤개수만큼 랜덤 방향으로 설정
    (bind _output_get_2 (Variables|Default|SetRandomRoom (Actor|GetComponentsByClass _output_get "/Script/Engine.ArrowComponent")))
    (Utilities|Array|Shuffle _output_get_2)
    (bind _output_get_3 (Variables|Default|SetRandomCount (.OutItem (Utilities|Array|Random (Utilities|Array|MakeArray 1 1 1 2 2 3)))))
    ;[0.15 0.15 0.15 0.5] 지정된 개수, 방향으로 각각 방 생성
    (for (_array_element _array_index) (Variables|Default|GetRandomRoom)
      ;[0.15 0.15 0.15 0.5] 검사
      (if (< _array_index _output_get_3)
        (Utilities|IsValid (Utilities|Array|Get(acopy) (Actor|GetComponentsbyTag (Variables|Default|GetProcessing%20Room) "/Script/Engine.StaticMeshComponent" (Utilities|Array|Get(acopy) (Variables|/Script/Engine.ActorComponent|GetComponentTags _array_element))))
          (:Is%20Valid
            ;[0.15 0.15 0.15 0.5] 충돌 검사
            (bind _returnvalue_2 (Collision|BoxOverlapActors (+ (.Location (Math|Transform|BreakTransform (Transformation|GetWorldTransform _array_element))) (* (Math|Vector|GetForwardVector (.Rotation (Math|Transform|BreakTransform (Transformation|GetWorldTransform _array_element)))) 2400)) "1500.000000,1500.000000,500.000000" (Utilities|Array|MakeArray "ObjectTypeQuery1" "ObjectTypeQuery2") 0 :!class /Script/Engine.KismetSystemLibrary))
            (if (not _returnvalue_2)
              ;[0.15 0.15 0.15 0.5] 만약 충돌이 없고 방을 만들 예정이라면 막고있던 문들 지우기
              (for _array_element_2 (Actor|GetComponentsbyTag (Variables|Default|GetProcessing%20Room) "/Script/Engine.StaticMeshComponent" (Utilities|Array|Get(acopy) (Variables|/Script/Engine.ActorComponent|GetComponentTags _array_element)))
                (Development|SetHiddeninGame _array_element_2 true false)
                (Collision|SetCollisionEnabled _array_element_2 "NoCollision"))
              ;[0.15 0.15 0.15 0.5] 터널 생성 후 위치정보 갱신
              (bind _returnvalue_3 (Game|SpawnActorfromClass "/Game/Levels/hyojun/3rd/BP_3rdPassRoom.BP_3rdPassRoom_C" (Transformation|GetWorldTransform _array_element) "Undefined" "MultiplyWithRoot" 0 0))
              ;[0.15 0.15 0.15 0.5] 방 개수 카운트 증가 및 만들 방 정보 갱신 후 전체 방 정보 저장
              (bind _returnvalue_4 (Game|SpawnActorfromClass "/Game/Levels/hyojun/3rd/BP_3rdCrossRoom.BP_3rdCrossRoom_C" (Transformation|GetWorldTransform (Variables|/Game/Levels/hyojun/BP_RoomMaster.BP_RoomMaster_C|GetExitPoint _returnvalue_3)) "AlwaysSpawn" "MultiplyWithRoot" 0 0))
              (Math|Integer|IncrementInt (Variables|Default|GetRoomCount)
                (:%20%20
                  (Utilities|Array|Add (Variables|Default|GetNextRoomList) _returnvalue_4)
                  (Utilities|Array|Add (Variables|Default|GetSpawnedRooms) _returnvalue_4)))))))))
  ;[0.15 0.15 0.15 0.5] 마지막 생성 방부터 하나씩 위치정보 가져오기, 보스 방 만들때까지 반복
  (bind _output_get_4 (Variables|Default|SetIsBossSpawned false))
  (bind _arrayelement (Utilities|Array|ReverseforEachLoop (Variables|Default|GetSpawnedRooms))
    (:LoopBody
      (if (not _output_get_4)
        ;[0.15 0.15 0.15 0.5] 보스방, 계단방 생성 전 충돌검사
        (bind _returnvalue_5 (Collision|BoxOverlapActors (+ (.Location (Math|Transform|BreakTransform (Transformation|GetWorldTransform (Utilities|Array|Get(acopy) (Actor|GetComponentsByClass _arrayelement "/Script/Engine.ArrowComponent"))))) (* (Math|Vector|GetForwardVector (.Rotation (Math|Transform|BreakTransform (Transformation|GetWorldTransform (Utilities|Array|Get(acopy) (Actor|GetComponentsByClass _arrayelement "/Script/Engine.ArrowComponent")))))) 3600)) "1500.000000,1500.000000,500.000000" (Utilities|Array|MakeArray "ObjectTypeQuery1" "ObjectTypeQuery2") 0 :!class /Script/Engine.KismetSystemLibrary))
        (if (not _returnvalue_5)
          ;[0.15 0.15 0.15 0.5] 보스 방 생성시 해당 방향에 있는 문 제거
          (Development|SetHiddeninGame (Utilities|Array|Get(acopy) (Actor|GetComponentsbyTag _arrayelement "/Script/Engine.StaticMeshComponent" (Utilities|Array|Get(acopy) (Variables|/Script/Engine.ActorComponent|GetComponentTags (Utilities|Array|Get(acopy) (Actor|GetComponentsByClass _arrayelement "/Script/Engine.ArrowComponent")))))) true false)
          (Collision|SetCollisionEnabled (Utilities|Array|Get(acopy) (Actor|GetComponentsbyTag _arrayelement "/Script/Engine.StaticMeshComponent" (Utilities|Array|Get(acopy) (Variables|/Script/Engine.ActorComponent|GetComponentTags (Utilities|Array|Get(acopy) (Actor|GetComponentsByClass _arrayelement "/Script/Engine.ArrowComponent")))))) "NoCollision")
          ;[0.15 0.15 0.15 0.5] 충돌이 없다면 통로 및 보스방 혹은 계단방 생성
          (bind _returnvalue_6 (Game|SpawnActorfromClass "/Game/Levels/hyojun/3rd/BP_3rdPassRoom.BP_3rdPassRoom_C" (Transformation|GetWorldTransform (Utilities|Array|Get(acopy) (Actor|GetComponentsByClass _arrayelement "/Script/Engine.ArrowComponent"))) "Undefined" "MultiplyWithRoot" 0 0))
          (Game|SpawnActorfromClass "/Game/Levels/hyojun/3rd/BP_3rdBossRomm.BP_3rdBossRomm_C" (Transformation|GetWorldTransform (Utilities|Array|Get(acopy) (Actor|GetComponentsByClass _returnvalue_6 "/Script/Engine.ArrowComponent"))) "Undefined" "MultiplyWithRoot" 0 0)
          (Variables|Default|SetIsBossSpawned true))))))

(event Collision|EventActorBeginOverlap
  (params (OtherActor :type Actor%20Object%20Reference)))

(event EventTick
  (params (DeltaSeconds :type Float%20%28single-precision%29)))

(fn ConstructionScript)