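; Test level actor that seeds the Mortis rune inventory for rune set synergy and slot testing.
; On BeginPlay it waits a tick, then binds to the inventory subsystem's owned, equipped and activated-set change events.
; A countdown loop then generates Common runes of one set tag through the rune database subsystem and adds them to the inventory.
; Nothing is equipped, and all event handlers are empty, with their debug prints disconnected.
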(event Custom|OnOwningRuneAdded_이벤트
  (params (RuneToAdd :type Mortis%20Rune%20Instance%20Structure%20%28by%20ref%29)))

(event Custom|OnOwningRuneRemoved_이벤트
  (params (RuneToRemove :type Mortis%20Rune%20Instance%20Structure%20%28by%20ref%29)))

(event Custom|OnEquippedRuneAdded_이벤트
  (params (SlotIndex :type Integer) (RuneToAdd :type Mortis%20Rune%20Instance%20Structure%20%28by%20ref%29)))

(event Custom|OnEquippedRuneRemoved_이벤트
  (params (SlotIndex :type Integer) (RuneToRemove :type Mortis%20Rune%20Instance%20Structure%20%28by%20ref%29)))

(event Custom|OnActivatedRuneSetsChanged_이벤트
  (params (ActiveRuneSetTags :type Array%20of%20Gameplay%20Tag%20Structures)))

(event EventBeginPlay
  (bind _returnvalue (Subsystems|GetMortisRuneInventorySubsystem))
  (Utilities|FlowControl|DelayUntilNextTick)
  (EventDispatchers|AssignOnOwningRuneAdded _returnvalue (delegate Custom|OnOwningRuneAdded_이벤트))
  (EventDispatchers|AssignOnOwningRuneRemoved _returnvalue (delegate Custom|OnOwningRuneRemoved_이벤트))
  (EventDispatchers|AssignOnEquippedRuneAdded _returnvalue (delegate Custom|OnEquippedRuneAdded_이벤트))
  (EventDispatchers|AssignOnEquippedRuneRemoved _returnvalue (delegate Custom|OnEquippedRuneRemoved_이벤트))
  (EventDispatchers|AssignOnActivatedRuneSetsChanged _returnvalue (delegate Custom|OnActivatedRuneSetsChanged_이벤트))
  ;[0.15 0.15 0.15 0.5] 룬 획득 및 장착
  (Variables|Default|SetRuneSpawnCount 10)
  (if (>= (Variables|Default|GetRuneSpawnCount) 0) :!label _label
    (Class|MortisRuneInventorySubsystem|AddRune (Subsystems|GetMortisRuneInventorySubsystem) (Class|MortisRuneDatabaseSubsystem|GenerateRunewithTag (Subsystems|GetMortisRuneDatabaseSubsystem) (Variables|Default|GetRuneSetToAdd1) "Common"))
    (Variables|Default|SetRuneSpawnCount (- (Variables|Default|GetRuneSpawnCount) 1))
    (goto _label)))

(fn ConstructionScript)