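; BP_ExperienceTest is a test Blueprint that exercises the Mortis meta-progression experience system on BeginPlay.
; It prints the Memory Fragments count, unlocks ExperienceTag if still locked, then selects it through MortisMetaProgressionSubsystem, printing "fail" if either step fails.
; On success it reads the selected experience row and applies only its first granted GameplayEffect to the player character's ability system component.
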(event EventBeginPlay
  (bind _returnvalue (Subsystems|GetMortisMetaProgressionSubsystem))
  (bind (_outrow _returnvalue_2) (Class|MortisMetaProgressionSubsystem|GetSelectedExperienceRow _returnvalue))
  (Development|PrintString (Utilities|String|ToString(Integer) (Class|MortisMetaProgressionSubsystem|GetMemoryFragments _returnvalue)))
  (if (Class|MortisMetaProgressionSubsystem|IsExperienceUnlocked _returnvalue (Variables|Default|GetExperienceTag))
    (bind _returnvalue_3 (Class|MortisMetaProgressionSubsystem|SelectExperience _returnvalue (Variables|Default|GetExperienceTag) :!label _label))
    (if _returnvalue_3
      (if _returnvalue_2
        (GameplayEffects|ApplyGameplayEffectToSelf :self (Variables|/Script/EternalMortis.MortisCharacterBase|GetMortisAbilitySystemComponent (.AsMortis%20Player%20Character (Utilities|Casting|CastToMortisPlayerCharacter (Game|Player|GetPlayerPawn 0)))) :GameplayEffectClass (Utilities|Array|Get(acopy) (.GrantedEffects (Utilities|Struct|BreakMortisExperienceRow _outrow)))))
      (else
        (Development|PrintString "fail" :!label _label_2)))
    (else
      (bind _returnvalue_4 (Class|MortisMetaProgressionSubsystem|UnlockExperience _returnvalue (Variables|Default|GetExperienceTag)))
      (if _returnvalue_4
        (goto _label)
        (else
          (goto _label_2))))))

(event Collision|EventActorBeginOverlap
  (params (OtherActor :type Actor%20Object%20Reference)))

(event EventTick
  (params (DeltaSeconds :type Float%20%28single-precision%29)))

(fn ConstructionScript)