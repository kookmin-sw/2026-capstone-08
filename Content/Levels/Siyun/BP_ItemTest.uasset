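; BP_ItemTest is a test actor that spawns a random weapon pickup at its own transform on BeginPlay.
; It asks the Mortis weapon database subsystem for random floor 6 weapons to fill the BP_WeaponPickup's data.
; It tints the pickup mesh's Fresnel color by weapon grade style.
; The data and tint come from separate generate calls, so the color may not match the weapon.
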(event EventBeginPlay
  (bind _returnvalue (Subsystems|GetMortisWeaponDatabaseSubsystem))
  (bind _outweaponrow (Class|MortisWeaponDatabaseSubsystem|GenerateRandomWeaponforFloor _returnvalue 6))
  (Variables|Default|SetOut%20Weapon%20Row _outweaponrow)
  (bind _returnvalue_2 (Game|SpawnActorfromClass "/Game/Items/PickUp/BP_WeaponPickup.BP_WeaponPickup_C" (Transformation|GetActorTransform) "Undefined" "MultiplyWithRoot" 0 0))
  (Class|MortisWeaponPickup|SetWeaponData _returnvalue_2 _outweaponrow)
  (Rendering|Material|SetColorParameterValueonMaterials (Variables|/Script/EternalMortis.MortisInteractableActorBase|GetVisualMesh _returnvalue_2) "FresColor" (.GradeColor (Utilities|Struct|BreakMortisWeaponGradeStyleRow (.OutStyleRow (Class|MortisWeaponDatabaseSubsystem|GetWeaponGradeStylebyHandle (Subsystems|GetMortisWeaponDatabaseSubsystem) (.GradeStyleRow (Utilities|Struct|BreakMortisWeaponRow (Variables|Default|GetOut%20Weapon%20Row)))))))))

(event Collision|EventActorBeginOverlap
  (params (OtherActor :type Actor%20Object%20Reference)))

(event EventTick
  (params (DeltaSeconds :type Float%20%28single-precision%29)))

(fn ConstructionScript)