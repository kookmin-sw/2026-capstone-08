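; BP_InvenTest is a test actor for the Mortis rune inventory subsystem.
; On BeginPlay it waits a tick, binds the inventory's add, remove, equip, unequip and active-set events, then generates six Common runes from one set tag, adding and equipping each in consecutive slots.
; The event handlers print rune IDs, slot indices and the activated set count.
; An unequip call is present but never runs.
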(event Custom|OnOwningRuneAdded_이벤트
  (params (RuneToAdd :type Mortis%20Rune%20Instance%20Structure%20%28by%20ref%29))
  (Development|PrintString (Utilities|String|Append "Add Inventory Rune ID : " (Guid|ToString(Guid) (.InstanceId (Utilities|Struct|BreakMortisRuneInstance RuneToAdd)))) true true "(R=0.000000,G=0.660000,B=1.000000,A=1.000000)" 1e+01))

(event Custom|OnOwningRuneRemoved_이벤트
  (params (RuneToRemove :type Mortis%20Rune%20Instance%20Structure%20%28by%20ref%29))
  (Development|PrintString (Utilities|String|Append "Remove InventoryRune ID : " (Guid|ToString(Guid) (.InstanceId (Utilities|Struct|BreakMortisRuneInstance RuneToRemove)))) true true "(R=0.000000,G=0.660000,B=1.000000,A=1.000000)" 1e+01))

(event Custom|OnEquippedRuneAdded_이벤트
  (params (SlotIndex :type Integer) (RuneToAdd :type Mortis%20Rune%20Instance%20Structure%20%28by%20ref%29))
  (Development|PrintString (Utilities|String|Append "Equip Slot Index : " (Utilities|String|ToString(Integer) SlotIndex)) true true "(R=0.000000,G=0.660000,B=1.000000,A=1.000000)" 1e+01)
  (Development|PrintString (Utilities|String|Append "Rune ID : " (Guid|ToString(Guid) (.InstanceId (Utilities|Struct|BreakMortisRuneInstance RuneToAdd)))) true true "(R=0.000000,G=0.660000,B=1.000000,A=1.000000)" 1e+01))

(event Custom|OnEquippedRuneRemoved_이벤트
  (params (SlotIndex :type Integer) (RuneToRemove :type Mortis%20Rune%20Instance%20Structure%20%28by%20ref%29))
  (Development|PrintString (Utilities|String|Append "Remove Slot Index : " (Utilities|String|ToString(Integer) SlotIndex)) true true "(R=0.000000,G=0.660000,B=1.000000,A=1.000000)" 1e+01)
  (Development|PrintString (Utilities|String|Append "Rune ID : " (Guid|ToString(Guid) (.InstanceId (Utilities|Struct|BreakMortisRuneInstance RuneToRemove)))) true true "(R=0.000000,G=0.660000,B=1.000000,A=1.000000)" 1e+01))

(event Custom|OnActivatedRuneSetsChanged_이벤트
  (params (ActiveRuneSetTags :type Array%20of%20Gameplay%20Tag%20Structures))
  (Development|PrintString (Utilities|String|Append (Utilities|String|ToString(Integer) (Utilities|Array|Length ActiveRuneSetTags)) " Set Activated") true true "(R=0.000000,G=0.660000,B=1.000000,A=1.000000)" 1e+01))

(event EventBeginPlay
  (bind _returnvalue (Subsystems|GetMortisRuneInventorySubsystem))
  (bind _returnvalue_2 (Subsystems|GetMortisRuneInventorySubsystem))
  (bind _returnvalue_3 (Subsystems|GetMortisRuneInventorySubsystem))
  (bind _returnvalue_4 (Subsystems|GetMortisRuneInventorySubsystem))
  (bind _returnvalue_5 (Subsystems|GetMortisRuneInventorySubsystem))
  (bind _returnvalue_6 (Subsystems|GetMortisRuneInventorySubsystem))
  (bind _returnvalue_7 (Subsystems|GetMortisRuneInventorySubsystem))
  (Utilities|FlowControl|DelayUntilNextTick)
  (EventDispatchers|AssignOnOwningRuneAdded _returnvalue (delegate Custom|OnOwningRuneAdded_이벤트))
  (EventDispatchers|AssignOnOwningRuneRemoved _returnvalue (delegate Custom|OnOwningRuneRemoved_이벤트))
  (EventDispatchers|AssignOnEquippedRuneAdded _returnvalue (delegate Custom|OnEquippedRuneAdded_이벤트))
  (EventDispatchers|AssignOnEquippedRuneRemoved _returnvalue (delegate Custom|OnEquippedRuneRemoved_이벤트))
  ;[0.15 0.15 0.15 0.5] 룬 획득 및 장착
  (EventDispatchers|AssignOnActivatedRuneSetsChanged _returnvalue (delegate Custom|OnActivatedRuneSetsChanged_이벤트))
  (bind _output_get (Variables|Default|SetTestRune1 (Class|MortisRuneDatabaseSubsystem|GenerateRunewithTag (Subsystems|GetMortisRuneDatabaseSubsystem) (Variables|Default|GetRuneSetToAdd1) "Common")))
  (Class|MortisRuneInventorySubsystem|AddRune _returnvalue_5 _output_get)
  (Class|MortisRuneInventorySubsystem|EquipRune _returnvalue_5 0 _output_get)
  (bind _output_get_2 (Variables|Default|SetTestRune2 (Class|MortisRuneDatabaseSubsystem|GenerateRunewithTag (Subsystems|GetMortisRuneDatabaseSubsystem) (Variables|Default|GetRuneSetToAdd1) "Common")))
  (Class|MortisRuneInventorySubsystem|AddRune _returnvalue_3 _output_get_2)
  (Class|MortisRuneInventorySubsystem|EquipRune _returnvalue_3 1 _output_get_2)
  (bind _output_get_3 (Variables|Default|SetTestRune3 (Class|MortisRuneDatabaseSubsystem|GenerateRunewithTag (Subsystems|GetMortisRuneDatabaseSubsystem) (Variables|Default|GetRuneSetToAdd1) "Common")))
  (Class|MortisRuneInventorySubsystem|AddRune _returnvalue_6 _output_get_3)
  (Class|MortisRuneInventorySubsystem|EquipRune _returnvalue_6 2 _output_get_3)
  (bind _output_get_4 (Variables|Default|SetTestRune4 (Class|MortisRuneDatabaseSubsystem|GenerateRunewithTag (Subsystems|GetMortisRuneDatabaseSubsystem) (Variables|Default|GetRuneSetToAdd1) "Common")))
  (Class|MortisRuneInventorySubsystem|AddRune _returnvalue_7 _output_get_4)
  (Class|MortisRuneInventorySubsystem|EquipRune _returnvalue_7 3 _output_get_4)
  (bind _output_get_5 (Variables|Default|SetTestRune5 (Class|MortisRuneDatabaseSubsystem|GenerateRunewithTag (Subsystems|GetMortisRuneDatabaseSubsystem) (Variables|Default|GetRuneSetToAdd1) "Common")))
  (Class|MortisRuneInventorySubsystem|AddRune _returnvalue_2 _output_get_5)
  (Class|MortisRuneInventorySubsystem|EquipRune _returnvalue_2 4 _output_get_5)
  (bind _output_get_6 (Variables|Default|SetTestRune6 (Class|MortisRuneDatabaseSubsystem|GenerateRunewithTag (Subsystems|GetMortisRuneDatabaseSubsystem) (Variables|Default|GetRuneSetToAdd1) "Common")))
  (Class|MortisRuneInventorySubsystem|AddRune _returnvalue_4 _output_get_6)
  (Class|MortisRuneInventorySubsystem|EquipRune _returnvalue_4 5 _output_get_6))

(event Collision|EventActorBeginOverlap
  (params (OtherActor :type Actor%20Object%20Reference)))

(event EventTick
  (params (DeltaSeconds :type Float%20%28single-precision%29)))

(fn ConstructionScript)