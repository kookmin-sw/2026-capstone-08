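; Base enemy projectile Blueprint that damages the player on impact.
; Its impact handler override casts the hit pawn to MortisPlayerCharacter and, on success, applies the projectile's damage effect spec to that pawn's Ability System Component.
; The handler returns true whether or not the cast succeeds, and the event graph holds only disabled default events.
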(event EventBeginPlay
  (|CallParentFunction) ; This node is disabled and will not be called.\nDrag off pins to build functionality.
)

(event Collision|EventActorBeginOverlap
  (params (OtherActor :type Actor%20Object%20Reference))
  (|CallParentFunction OtherActor) ; This node is disabled and will not be called.\nDrag off pins to build functionality.
)

(event EventTick
  (params (DeltaSeconds :type Float%20%28single-precision%29))
  (|CallParentFunction DeltaSeconds) ; This node is disabled and will not be called.\nDrag off pins to build functionality.
)

(fn ConstructionScript
  (|CallParentFunction))

(fn BPHandleProjectileImpact
  (params (HitPawn :type Pawn%20Object%20Reference) (HitResult :type Hit%20Result%20Structure%20%28by%20ref%29) (Payload :type Gameplay%20Event%20Data%20Structure%20%28by%20ref%29))
  (Utilities|Casting|CastToMortisPlayerCharacter HitPawn
    (:then
      (GameplayEffects|ApplyGameplayEffectSpecToSelf (Ability|GetAbilitySystemComponent HitPawn) (Variables|Default|GetProjectileDamageEffectSpecHandle)))
    (:CastFailed
      _))
  (return true))