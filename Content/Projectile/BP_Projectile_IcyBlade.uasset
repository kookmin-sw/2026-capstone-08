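; Icy Blade projectile Blueprint that applies GAS-based damage to the pawn it hits.
; Its impact handler override applies the projectile's damage effect spec to the hit pawn's Ability System Component and always returns true, leaving the hit result and payload unused.
; The event graph holds only disabled default events, and the construction script just calls its parent.
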(event EventBeginPlay
  (|CallParentFunction) ; 지금 이 노드는 비활성 상태입니다. \n핀을 끌어서 다른 노드를 연결하면 활성화됩니다.
)

(event Collision|EventActorBeginOverlap
  (params (OtherActor :type Actor%20Object%20Reference))
  (|CallParentFunction OtherActor) ; 지금 이 노드는 비활성 상태입니다. \n핀을 끌어서 다른 노드를 연결하면 활성화됩니다.
)

(event EventTick
  (params (DeltaSeconds :type Float%20%28single-precision%29))
  (|CallParentFunction DeltaSeconds) ; 지금 이 노드는 비활성 상태입니다. \n핀을 끌어서 다른 노드를 연결하면 활성화됩니다.
)

(fn ConstructionScript
  (|CallParentFunction))

(fn BPHandleProjectileImpact
  (params (HitPawn :type Pawn%20Object%20Reference) (HitResult :type Hit%20Result%20Structure%20%28by%20ref%29) (Payload :type Gameplay%20Event%20Data%20Structure%20%28by%20ref%29))
  (GameplayEffects|ApplyGameplayEffectSpecToSelf (Ability|GetAbilitySystemComponent HitPawn) (Variables|Default|GetProjectileDamageEffectSpecHandle))
  (return true))