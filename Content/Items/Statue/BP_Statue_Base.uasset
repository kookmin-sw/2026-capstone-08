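; BP_Statue_Base is a base statue actor that grants random runes and may inflict a curse.
; The Construction Script gathers three item points, and GiveItems spawns a rune pickup at the statue mesh for each, dropped toward that point.
; Runes are generated from the statue's RuneTag through the rune database subsystem and tinted by grade color.
; GiveItems then finishes the interaction and randomly adds a curse through the curse inventory subsystem.
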(event EventBeginPlay)

(event Collision|EventActorBeginOverlap
  (params (OtherActor :type Actor%20Object%20Reference)))

(event EventTick
  (params (DeltaSeconds :type Float%20%28single-precision%29)))

(fn ConstructionScript
  (bind _itempoints (Variables|Default|GetItemPoints))
  (Utilities|Array|Clear _itempoints)
  (Utilities|Array|Add _itempoints (Variables|Default|GetItemPoint1))
  (Utilities|Array|Add _itempoints (Variables|Default|GetItemPoint2))
  (Utilities|Array|Add _itempoints (Variables|Default|GetItemPoint3)))

(fn GiveItems
  (bind _visualmesh (Variables|Default|GetVisualMesh))
  (bind _returnvalue (Transformation|GetWorldTransform _visualmesh))
  (for _index (range 0 (- (Utilities|Array|Length (Variables|Default|GetItemPoints)) 1))
    (bind _returnvalue_2 (Game|SpawnActorfromClass "/Game/Items/PickUp/BP_RunePickup.BP_RunePickup_C" (Math|Transform|MakeTransform (.location _returnvalue) (.rotation _returnvalue) "1.000000,1.000000,1.000000") "Undefined" "MultiplyWithRoot" 0 0))
    (Class|MortisRunePickup|ReactivateasDroppedRune _returnvalue_2 (Class|MortisRuneDatabaseSubsystem|GenerateRandomRunewithTag (Subsystems|GetMortisRuneDatabaseSubsystem) (Variables|Default|GetRuneTag) 1) (Transformation|GetActorLocation _returnvalue_2) (Transformation|GetWorldLocation (Utilities|Array|Get(acopy) (Variables|Default|GetItemPoints) _index)) -1.0 -1.0)
    (Rendering|Material|SetColorParameterValueonMaterials (Variables|/Script/EternalMortis.MortisInteractableActorBase|GetVisualMesh _returnvalue_2) "FresColor" (.GradeColor (Utilities|Struct|BreakMortisRuneGradeStyleRow (.OutStyleRow (Class|MortisRuneDatabaseSubsystem|GetRuneGradeStylebyHandle (Subsystems|GetMortisRuneDatabaseSubsystem) (.GradeStyleRow (Utilities|Struct|BreakMortisRuneInstance (Variables|/Script/EternalMortis.MortisRunePickup|GetRuneData _returnvalue_2))))))))
    (Transformation|SetActorRotation _returnvalue_2 (Transformation|GetWorldRotation (Utilities|Array|Get(acopy) (Variables|Default|GetItemPoints) _index))))
  (Class|MortisInteractableActorBase|OnInteractionFinished 0 true)
  (if (Math|Random|RandomBool)
    (Class|MortisCurseInventorySubsystem|GenerateandAddCurse (Subsystems|GetMortisCurseInventorySubsystem))))