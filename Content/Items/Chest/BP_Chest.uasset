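; BP_Chest is a loot chest that swings open and drops randomly generated runes and a weapon.
; OpenChest plays a timeline that pitches the lid pivot, then calls CreateItems and reports the interaction finished.
; CreateItems spawns one or two rune pickups and one weapon pickup from database subsystems, tinting each by grade color.
; Each pickup is dropped toward a random line-traced ground point in front of the chest.
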(event Custom|OpenChest
  (bind _headdegree (Timeline|TL_OpeningChest Play)
    (:Update
      (Transformation|SetRelativeRotation (Variables|Default|GetPivot) (Math|Rotator|MakeRotator 0.0 _headdegree 0.0) false false))
    (:Finished
      (CallFunction|CreateItems)
      (Class|MortisInteractableActorBase|OnInteractionFinished 0 true))))

(event EventBeginPlay)

(event Collision|EventActorBeginOverlap
  (params (OtherActor :type Actor%20Object%20Reference)))

(event EventTick
  (params (DeltaSeconds :type Float%20%28single-precision%29)))

(fn ConstructionScript)

(fn GetRandomGroundPoint
  (bind _returnvalue (Transformation|GetActorForwardVector))
  (LocalVariables|SetCenter (+ (Transformation|GetActorLocation) (* _returnvalue (LocalVariables|GetForwardDistance))))
  (bind _output_get (LocalVariables|SetCandidate (+ (* _returnvalue (* (Math|Trig|Sin(Degrees) (Math|Random|RandomFloatinRange 0.0 3.6e+02)) (Math|Random|RandomFloatinRange 0.0 (LocalVariables|GetRadius)))) (+ (LocalVariables|GetCenter) (* (Transformation|GetActorRightVector) (* (Math|Trig|Cos(Degrees) (Math|Random|RandomFloatinRange 0.0 3.6e+02)) (Math|Random|RandomFloatinRange 0.0 (LocalVariables|GetRadius))))))))
  (bind _outhit (Collision|LineTraceForObjects (+ _output_get "0.000000,0.000000,200.000000") (+ _output_get "0.000000,0.000000,-200.000000") (LocalVariables|GetObjectTypes) false 0 "None"))
  (return (.ImpactPoint (Collision|BreakHitResult _outhit))))

(fn CreateItems
  (Utilities|FlowControl|Sequence
    (:then_0
      (for _index (range 0 (Math|Random|RandomIntegerinRange 1 2))
        (bind _output_get (LocalVariables|SetCachedRandomRune (Class|MortisRuneDatabaseSubsystem|GenerateRune (Subsystems|GetMortisRuneDatabaseSubsystem) 1)))
        (bind _returnvalue (Game|SpawnActorfromClass "/Game/Items/PickUp/BP_RunePickup.BP_RunePickup_C" (Transformation|GetActorTransform) "Undefined" "MultiplyWithRoot" 0 0))
        (Transformation|SetActorRotation _returnvalue (Math|Rotator|MakeRotator 0.0 0.0 (.yaw (Math|Random|RandomRotator false))))
        (bind _outposition (CallFunction|GetRandomGroundPoint))
        (Class|MortisRunePickup|ReactivateasDroppedRune _returnvalue _output_get (Transformation|GetActorLocation _returnvalue) _outposition -1.0 -1.0)
        (Rendering|Material|SetColorParameterValueonMaterials (Variables|/Script/EternalMortis.MortisPickupBase|GetSelectionIndicatorMesh _returnvalue) "FresColor" (.GradeColor (Utilities|Struct|BreakMortisRuneGradeStyleRow (.OutStyleRow (Class|MortisRuneDatabaseSubsystem|GetRuneGradeStylebyHandle (Subsystems|GetMortisRuneDatabaseSubsystem) (.GradeStyleRow (Utilities|Struct|BreakMortisRuneInstance (Variables|/Script/EternalMortis.MortisRunePickup|GetRuneData _returnvalue))))))))))
    (:then_1
      (bind _output_get_2 (LocalVariables|SetCachedRandomWeapon (.OutWeaponRow (Class|MortisWeaponDatabaseSubsystem|GenerateRandomWeaponforFloor (Subsystems|GetMortisWeaponDatabaseSubsystem) 1))))
      (bind _returnvalue_2 (Game|SpawnActorfromClass "/Game/Items/PickUp/BP_WeaponPickup.BP_WeaponPickup_C" (Transformation|GetActorTransform) "Undefined" "MultiplyWithRoot" 0 0))
      (Transformation|SetActorRotation _returnvalue_2 (Math|Rotator|MakeRotator 0.0 0.0 (.yaw (Math|Random|RandomRotator false))))
      (bind _outposition_2 (CallFunction|GetRandomGroundPoint))
      (Class|MortisWeaponPickup|ReactivateasDroppedWeapon _returnvalue_2 _output_get_2 (Transformation|GetActorLocation _returnvalue_2) _outposition_2 -1.0 -1.0)
      (Rendering|Material|SetColorParameterValueonMaterials (Variables|/Script/EternalMortis.MortisInteractableActorBase|GetVisualMesh _returnvalue_2) "FresColor" (.GradeColor (Utilities|Struct|BreakMortisWeaponGradeStyleRow (.OutStyleRow (Class|MortisWeaponDatabaseSubsystem|GetWeaponGradeStylebyHandle (Subsystems|GetMortisWeaponDatabaseSubsystem) (.GradeStyleRow (Utilities|Struct|BreakMortisWeaponRow (LocalVariables|GetCachedRandomWeapon)))))))))))