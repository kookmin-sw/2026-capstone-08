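; BP_StairGate is a stair gate that moves the player to the next floor or to an ending level on overlap.
; Below floor 6 it increments CurrentFloor in MortisGameInstance, advances CurrentConcept on reaching floors 3 and 5, and opens that floor's level.
; On floor 6 it opens TrueEnding with three or more owned curses, otherwise End.
; DoOnce precedes the player cast, so any actor's first overlap consumes it.
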(event EventBeginPlay
  (|CallParentFunction) ; 지금 이 노드는 비활성 상태입니다. \n핀을 끌어서 다른 노드를 연결하면 활성화됩니다.
)

(event Collision|EventActorBeginOverlap
  (params (OtherActor :type Actor%20Object%20Reference))
  (|CallParentFunction OtherActor)
  (Utilities|FlowControl|DoOnce false
    (:Completed
      (Utilities|Casting|CastToBP_PlayerCharacter OtherActor)
      (bind _asmortis_game_instance (Utilities|Casting|CastToMortisGameInstance (Game|GetGameInstance)))
      (if (== (Variables|/Script/EternalMortis.MortisGameInstance|GetCurrentFloor _asmortis_game_instance) 6)
        (if (>= (Utilities|Array|Length (Class|MortisCurseInventorySubsystem|GetOwnedCurses (Subsystems|GetMortisCurseInventorySubsystem))) 3)
          (Development|PrintString "진엔딩")
          (Game|OpenLevel(byName) "/Game/Levels/hyojun/RealBoss/TrueEnding.TrueEnding")
          (else
            (Development|PrintString "일반엔딩")
            (Game|OpenLevel(byName) "/Game/Levels/hyojun/RealBoss/End.End")))
        (else
          (bind _output_get (Variables|/Script/EternalMortis.MortisGameInstance|SetCurrentFloor _asmortis_game_instance (+ (Variables|/Script/EternalMortis.MortisGameInstance|GetCurrentFloor _asmortis_game_instance) 1)))
          (if (or (== _output_get 3) (== _output_get 5))
            (Variables|/Script/EternalMortis.MortisGameInstance|SetCurrentConcept _asmortis_game_instance (+ (Variables|/Script/EternalMortis.MortisGameInstance|GetCurrentConcept _asmortis_game_instance) 1)))
          (Game|OpenLevel(byName) (Utilities|Select :Index _output_get :Option%200 "" :Option%201 "/Game/Levels/hyojun/1st/nolight1.nolight" :Option%202 "/Game/Levels/hyojun/1st/nolight1.nolight1" :Option%203 "/Game/Levels/hyojun/2nd/withlight.withlight" :Option%204 "/Game/Levels/hyojun/2nd/withlight.withlight1" :Option%205 "/Game/Levels/hyojun/3rd/necroTest.necroTest" :Option%206 "/Game/Levels/hyojun/3rd/necroTest.necroTest1")))))))

(event EventTick
  (params (DeltaSeconds :type Float%20%28single-precision%29))
  (|CallParentFunction DeltaSeconds) ; 지금 이 노드는 비활성 상태입니다. \n핀을 끌어서 다른 노드를 연결하면 활성화됩니다.
)

(fn ConstructionScript
  (|CallParentFunction))