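; BP_TutoGate is a gate, likely for the tutorial, that opens another level when the player overlaps it.
; On overlap it calls the parent handler, passes a DoOnce, then checks for BP_PlayerCharacter and MortisGameInstance before opening the level.
; The level Select has a fixed index, so it always loads nolight1.
; DoOnce precedes the player check, so any first overlapping actor uses up the trigger.
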(event EventBeginPlay
  (|CallParentFunction) ; 지금 이 노드는 비활성 상태입니다. \n핀을 끌어서 다른 노드를 연결하면 활성화됩니다.
)

(event Collision|EventActorBeginOverlap
  (params (OtherActor :type Actor%20Object%20Reference))
  (|CallParentFunction OtherActor)
  (Utilities|FlowControl|DoOnce false
    (:Completed
      (Utilities|Casting|CastToBP_PlayerCharacter OtherActor)
      (Utilities|Casting|CastToMortisGameInstance (Game|GetGameInstance))
      (Game|OpenLevel(byName) (Utilities|Select :Index 0 :Option%200 "/Game/Levels/hyojun/1st/nolight1.nolight" :Option%201 "" :Option%202 "" :Option%203 "" :Option%204 "" :Option%205 "" :Option%206 "")))))

(event EventTick
  (params (DeltaSeconds :type Float%20%28single-precision%29))
  (|CallParentFunction DeltaSeconds) ; 지금 이 노드는 비활성 상태입니다. \n핀을 끌어서 다른 노드를 연결하면 활성화됩니다.
)

(fn ConstructionScript
  (|CallParentFunction))