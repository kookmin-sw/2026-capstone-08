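; BP_DragonSwordSpawn is a sword skill actor that reports hits on enemies entering its Box collision.
; On overlap, it sends an Event.Combat.AttackHit gameplay event to its Instigator with the MortisEnemyCharacter as target.
; EnemySet limits this to one hit per enemy until ResetEnemySet clears it.
; The construction script tints the static mesh's FresColor material parameter red.
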(event OnComponentBeginOverlap(Box)
  (params (OverlappedComponent :type Primitive%20Component%20Object%20Reference) (OtherActor :type Actor%20Object%20Reference) (OtherComp :type Primitive%20Component%20Object%20Reference) (OtherBodyIndex :type Integer) (bFromSweep :type Boolean) (SweepResult :type Hit%20Result%20Structure%20%28by%20ref%29))
  (bind _asmortis_enemy_character (Utilities|Casting|CastToMortisEnemyCharacter OtherActor))
  (Utilities|IsValid _asmortis_enemy_character
    (:Is%20Valid
      (if (not (Utilities|Set|Contains (Variables|Default|GetEnemySet) _asmortis_enemy_character))
        (Ability|SendGameplayEventtoActor (Variables|Actor|GetInstigator) "(TagName=\"Event.Combat.AttackHit\")" (Utilities|Struct|MakeGameplayEventData "(TagName=\"Event.Combat.AttackHit\")" 0 _asmortis_enemy_character))
        (Utilities|Set|Add (Variables|Default|GetEnemySet) _asmortis_enemy_character)))))

(event EventBeginPlay)

(event Collision|EventActorBeginOverlap
  (params (OtherActor :type Actor%20Object%20Reference)))

(event EventTick
  (params (DeltaSeconds :type Float%20%28single-precision%29)))

(fn ConstructionScript
  (Rendering|Material|SetColorParameterValueonMaterials (Variables|Default|GetStaticMesh) "FresColor" "(R=1.000000,G=0.060556,B=0.000000,A=1.000000)"))

(fn ResetEnemySet
  (Utilities|Set|Clear (Variables|Default|GetEnemySet)))